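; Grenade projectile that flies straight ahead and spawns an explosion when it is hit.
; Tick moves it manually along its forward vector from the mesh's world transform, without sweep or gravity, at a base speed that SetMuzzleVel multiplies.
; On Hit, if its owner is PlayerCharacterBP, it spawns GrenadeExplode with that instigator, passes itself via GetActors, then destroys itself.
; Its short lifespan removes it without exploding.
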(event EventSetMuzzleVel
  (params (vel :type Float%20%28single-precision%29))
  (Variables|Default|Setvelocity (* vel (Variables|Default|Getvelocity))))

(event EventBeginPlay)

(event EventActorBeginOverlap
  (params (OtherActor :type Actor%20Object%20Reference)))

(event EventTick
  (params (DeltaSeconds :type Float%20%28single-precision%29))
  (CallFunction|Move DeltaSeconds))

(event Collision|EventHit
  (params (MyComp :type Primitive%20Component%20Object%20Reference) (Other :type Actor%20Object%20Reference) (OtherComp :type Primitive%20Component%20Object%20Reference) (bSelfMoved :type Boolean) (HitLocation :type Vector :default "0, 0, 0") (HitNormal :type Vector :default "0, 0, 0") (NormalImpulse :type Vector :default "0, 0, 0") (Hit :type Hit%20Result%20Structure%20%28by%20ref%29))
  (bind _asplayer_character_bp (Utilities|Casting|CastToPlayerCharacterBP (Components|GetOwner)))
  (bind _returnvalue (Game|SpawnActorfromClass "/Game/Weapon/Ammo/Grenade/GrenadeExplode.GrenadeExplode_C" (Transformation|GetActorTransform) "Undefined" 0 _asplayer_character_bp))
  (Default|GetActors _returnvalue self)
  (Actor|DestroyActor))

(fn ConstructionScript
  (Variables|Default|Setvelocity 7e+02)
  (Actor|SetLifeSpan 5.0))

(fn Move
  (params (Delta :type Float%20%28single-precision%29))
  (bind _staticmesh (Variables|Default|GetStaticMesh))
  (bind _returnvalue (Transformation|GetWorldTransform _staticmesh))
  (bind (_location _rotation _scale) (Math|Transform|BreakTransform _returnvalue))
  (Transformation|SetActorTransform (Math|Transform|MakeTransform (+ (* (Transformation|GetActorForwardVector) (* Delta (Variables|Default|Getvelocity))) _location) _rotation _scale)))