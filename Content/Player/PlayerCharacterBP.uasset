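; Player character Blueprint that handles dual-trigger shooting, health, death and pausing.
; On BeginPlay it spawns a gun attached to the spring arm and adds the HUD, then forwards left and right fire inputs to the gun's triggers.
; Damage or a fall sets a Dead flag, which Tick polls to destroy the actor, pause and show the death screen.
; A separate pause event pauses the game and shows the pause menu.
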(event EventOnShootPressedLeft
  (Class|PlayerGun|PullTrigger (Variables|Default|GetPlayersGun) true))

(event EventOnShootReleasedLeft
  (Class|PlayerGun|ReleaseTrigger (Variables|Default|GetPlayersGun) true))

(event EventOnShootPressedRight
  (Class|PlayerGun|PullTrigger (Variables|Default|GetPlayersGun) false))

(event EventOnShootReleasedRight
  (Class|PlayerGun|ReleaseTrigger (Variables|Default|GetPlayersGun) false))

(event EventPauseGame
  (bind _returnvalue (Game|GetPlayerController 0))
  (Game|SetGamePaused true)
  (Input|SetInputModeUIOnly 0 (Variables|Default|GetPauseMenuVar) true)
  (Variables|/Script/Engine.PlayerController|SetbShowMouseCursor _returnvalue true)
  (Utilities|IsValid (Variables|Default|GetPauseMenuVar)
    (:Is%20Valid
      _)
    (:Is%20Not%20Valid
      (bind _returnvalue_2 (UserInterface|CreateWidget "/Game/UI/Pause.Pause_C" _returnvalue))
      (Variables|Default|SetPauseMenuVar _returnvalue_2)))
  (UserInterface|Viewport|AddtoViewport (Variables|Default|GetPauseMenuVar) 0))

(event EventFell
  (Variables|Default|SetDead true))

(event EventBeginPlay
  (bind _returnvalue (Game|SpawnActorfromClass "/Game/Weapon/TheGun/PlayerGunBP.PlayerGunBP_C" (Transformation|GetActorTransform) "Undefined" 0 0))
  (bind _output_get (Variables|Default|SetPlayersGun _returnvalue))
  (Class|Actor|AttachRootComponentto _output_get (Variables|Default|GetSpringArm) "None" "SnapToTarget" true)
  (bind _returnvalue_2 (UserInterface|CreateWidget "/Game/UI/PlayerUI.PlayerUI_C" (Game|GetPlayerController 0)))
  (bind _output_get_2 (Variables|Default|SetUI%20Var _returnvalue_2))
  (UserInterface|Viewport|AddtoViewport _output_get_2 0)
  (Actor|SetOwner (Variables|Default|GetPlayersGun) self))

(event Game|Damage|EventAnyDamage
  (params (Damage :type Float%20%28single-precision%29) (DamageType :type Damage%20Type%20Object%20Reference) (InstigatedBy :type Controller%20Object%20Reference) (DamageCauser :type Actor%20Object%20Reference))
  (bind _output_get (Variables|Default|SetHealth (- (Variables|Default|GetHealth) Damage)))
  (if (<= (Math|Float|Truncate (* _output_get 1e+02)) 0)
    (Variables|Default|SetDead true)))

(event EventActorBeginOverlap
  (params (OtherActor :type Actor%20Object%20Reference)))

(event EventTick
  (params (DeltaSeconds :type Float%20%28single-precision%29))
  (if (Variables|Default|GetDead)
    (Actor|DestroyActor)
    (Game|SetGamePaused true)
    (Utilities|IsValid (Variables|Default|GetDeadUI)
      (:Is%20Valid
        _)
      (:Is%20Not%20Valid
        (bind _returnvalue (UserInterface|CreateWidget "/Game/UI/DeadUI.DeadUI_C"))
        (Variables|Default|SetDeadUI _returnvalue)))
    (UserInterface|Viewport|AddtoViewport (Variables|Default|GetDeadUI) 0)
    (Variables|/Script/Engine.PlayerController|SetbShowMouseCursor (Game|GetPlayerController 0) true)))

(fn ConstructionScript
  (Variables|Default|SetHealth 1.0)
  (Variables|Default|SetDead false)
  (Variables|Default|SetKills 0))